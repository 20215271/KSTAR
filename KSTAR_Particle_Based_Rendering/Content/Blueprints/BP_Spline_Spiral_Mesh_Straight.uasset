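; BP_Spline_Spiral_Mesh_Straight is a procedural actor that builds a helix of straight spline mesh segments in its Construction Script.
; SpiralSplineCoord computes helix points from point count, angle step, radius and height per turn.
; These points rebuild the Spline with zero tangents, giving straight segments between neighbors.
; The spline mesh loop is nested inside the point loop, so segments are added again for every point.
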(fn `SpiralSplineCoord`
  (bind _radius (`self.Radius`))
  (for _index (range (`self.NumberOfPoints`))
    (bind _returnvalue (`KismetMathLibrary.DegreesToRadians` (* _index (`self.Angle`))))
    (`KismetArrayLibrary.Array_Add` (`self.VectorArray`) (`KismetMathLibrary.MakeVector` (* (`KismetMathLibrary.Cos` _returnvalue) _radius) (* (`KismetMathLibrary.Sin` _returnvalue) _radius) (`KismetMathLibrary.Conv_IntToDouble` (* _index (/ (`self.Heights`) (/ 360.0 (`self.Angle`)))))))))

(fn `UserConstructionScript`
  (bind _returnvalue (`KismetMathLibrary.Vector_Zero`))
  (bind _spline (`self.Spline`))
  (bind _spline_2 (`self.Spline`))
  (`self.SpiralSplineCoord`)
  (`SplineComponent.ClearSplinePoints` _spline true)
  (for (_array_element _array_index) (`self.VectorArray`)
    (`SplineComponent.AddSplinePoint` _spline _array_element "Local" true)
    (`SplineComponent.SetTangentAtSplinePoint` (`self.Spline`) _array_index (`KismetMathLibrary.Vector_Zero`) "Local" true)
    (for _index (range (+ (- (`KismetArrayLibrary.Array_Length` (`self.VectorArray`)) 2) 1))
      (bind _returnvalue_2 (`AddComponent|NODE_AddSplineMeshComponent-2`))
      (`SplineMeshComponent.SetStartAndEnd` _returnvalue_2 (`SplineComponent.GetLocationAtSplinePoint` _spline_2 _index "Local") _returnvalue (`SplineComponent.GetLocationAtSplinePoint` _spline_2 (+ _index 1) "Local") _returnvalue true))))