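; BP_Dissolve is an actor whose Cube component defines an oriented box volume for a dissolve effect through the MPC_Dissolve material parameter collection.
; The construction script writes the cube's world location, world scale (as Bounds) and forward, right and up vectors into the collection.
; The event graph is empty, so nothing updates at runtime, and all instances write to the same shared parameters.
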(fn `UserConstructionScript`
  (bind _cube (`self.Cube`))
  (`KismetMaterialLibrary.SetVectorParameterValue` "/Game/Materials/MPC_Dissolve.MPC_Dissolve" "Location" (`KismetMathLibrary.Conv_VectorToLinearColor` (`SceneComponent.K2_GetComponentLocation` _cube)))
  (`KismetMaterialLibrary.SetVectorParameterValue` "/Game/Materials/MPC_Dissolve.MPC_Dissolve" "Bounds" (`KismetMathLibrary.Conv_VectorToLinearColor` (`SceneComponent.K2_GetComponentScale` _cube)))
  (`KismetMaterialLibrary.SetVectorParameterValue` "/Game/Materials/MPC_Dissolve.MPC_Dissolve" "X" (`KismetMathLibrary.Conv_VectorToLinearColor` (`SceneComponent.GetForwardVector` _cube)))
  (`KismetMaterialLibrary.SetVectorParameterValue` "/Game/Materials/MPC_Dissolve.MPC_Dissolve" "Y" (`KismetMathLibrary.Conv_VectorToLinearColor` (`SceneComponent.GetRightVector` _cube)))
  (`KismetMaterialLibrary.SetVectorParameterValue` "/Game/Materials/MPC_Dissolve.MPC_Dissolve" "Z" (`KismetMathLibrary.Conv_VectorToLinearColor` (`SceneComponent.GetUpVector` _cube))))