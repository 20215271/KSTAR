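; Construction-script actor that builds a helical spiral of spline meshes, with point count, angle step, radius and rise per turn as variables.
; SpiralSplineCoord fills VectorArray using cosine and sine for the circle and a linear Z climb.
; The construction script rebuilds the Spline from those points, adding spline mesh components that follow segment positions and tangents.
; The segment loop is nested inside the point loop, so it repeats for every added point.
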(fn `SpiralSplineCoord`
  (bind _radius (`self.Radius`))
  (for _index (range (`self.NumberOfPoints`))
    (bind _returnvalue (`KismetMathLibrary.DegreesToRadians` (* _index (`self.Angle`))))
    (`KismetArrayLibrary.Array_Add` (`self.VectorArray`) (`KismetMathLibrary.MakeVector` (* (`KismetMathLibrary.Cos` _returnvalue) _radius) (* (`KismetMathLibrary.Sin` _returnvalue) _radius) (`KismetMathLibrary.Conv_IntToDouble` (* _index (/ (`self.Heights`) (/ 360.0 (`self.Angle`)))))))))

(fn `UserConstructionScript`
  (bind _spline (`self.Spline`))
  (`self.SpiralSplineCoord`)
  (`SplineComponent.ClearSplinePoints` _spline true)
  (for _array_element (`self.VectorArray`)
    (`SplineComponent.AddSplinePoint` _spline _array_element "Local" true)
    (for _index (range (+ (- (`KismetArrayLibrary.Array_Length` (`self.VectorArray`)) 2) 1))
      (bind _returnvalue (`AddComponent|NODE_AddSplineMeshComponent-2`))
      (bind _returnvalue_2 (+ _index 1))
      (`SplineMeshComponent.SetStartAndEnd` _returnvalue (`SplineComponent.GetLocationAtSplinePoint` (`self.Spline`) _index "Local") (`SplineComponent.GetTangentAtSplinePoint` (`self.Spline`) _index "Local") (`SplineComponent.GetLocationAtSplinePoint` (`self.Spline`) _returnvalue_2 "Local") (`SplineComponent.GetTangentAtSplinePoint` (`self.Spline`) _returnvalue_2 "Local") true))))