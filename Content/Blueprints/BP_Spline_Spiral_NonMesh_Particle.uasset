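; Spiral spline actor with a particle system meant to loop along the helix.
; The construction script builds the spline from points computed by SpiralSplineCoord using point count, angle step, radius and height per turn.
; The ParticleMovement timeline maps Distance to spline length, passing local positions as world locations, and restarts the particle at each end.
; Nothing starts that timeline, so the movement logic never runs.
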(fn `SpiralSplineCoord`
  (bind _radius (`self.Radius`))
  (for _index (range (`self.NumberOfPoints`))
    (bind _returnvalue (`KismetMathLibrary.DegreesToRadians` (* _index (`self.Angle`))))
    (`KismetArrayLibrary.Array_Add` (`self.VectorArray`) (`KismetMathLibrary.MakeVector` (* (`KismetMathLibrary.Cos` _returnvalue) _radius) (* (`KismetMathLibrary.Sin` _returnvalue) _radius) (`KismetMathLibrary.Conv_IntToDouble` (* _index (/ (`self.Heights`) (/ 360.0 (`self.Angle`)))))))))

(fn `UserConstructionScript`
  (bind _spline (`self.Spline`))
  (`self.SpiralSplineCoord`)
  (`SplineComponent.ClearSplinePoints` _spline true)
  (for _array_element (`self.VectorArray`)
    (`SplineComponent.AddSplinePoint` _spline _array_element "Local" true)))